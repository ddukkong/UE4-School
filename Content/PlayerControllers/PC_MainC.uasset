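; Player controller that gives each player an on-screen chat box and a stored player name.
; On BeginPlay it sets game-only input and adds a W_Chat widget to the viewport; Enter switches to game-and-UI input focused on the chat with the cursor visible.
; ServerSendMessage hands sender and text to MainGameMode to send to everyone, while AddMessageToChat appends a message to the widget's list.
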(event `self.ReceiveBeginPlay`
  (`WidgetBlueprintLibrary.SetInputMode_GameOnly` (`GameplayStatics.GetPlayerController` 0))
  (`self.CreateChatWidget`))

(event `CreateChatWidget`
  ;[1 1 1] Chatting
  (bind _returnvalue (`|CreateWidget` "/Game/Widgets/W_Chat.W_Chat_C"))
  (bind _output_get (set `self.W Chat` _returnvalue))
  (`UserWidget.AddToViewport` _output_get 0))

(event `Show Chat`
  ;[1 1 1] Chatting
  (`WidgetBlueprintLibrary.SetInputMode_GameAndUIEx` self (`self.W Chat`))
  (set `self.bShowMouseCursor` true))

(event `SetPlayerName`
  (params (NewName :type String))
  ;[1 1 1] Chatting
  (set `self.PlayerName` NewName))

(event `Key|Enter`
  (params (Key :type "Key Structure"))
  ;[1 1 1] Chatting
  (:`Pressed`
    (`self.ShowChat`)))

(event `ServerSendMessage`
  (params (Sender :type String) (Message :type String))
  ;[1 1 1] Chatting
  (bind _asmain_game_mode (cast `/Game/Gamemodes/MainGameMode` (`GameplayStatics.GetGameMode`)))
  (`/Game/Gamemodes/MainGameMode.SendMessagesToEveryone` _asmain_game_mode Sender Message))

(event `AddMessageToChat`
  (params (Sender :type String) (Message :type String))
  ;[1 1 1] Chatting
  (`/Game/Widgets/W_Chat.AddMessageOntoMessageList` (`self.W Chat`) Sender Message))

(fn `ShowChat`)

(fn `UserConstructionScript`)