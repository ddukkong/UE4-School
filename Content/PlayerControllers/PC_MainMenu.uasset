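; Main menu player controller that shows the menu UI and forwards session hosting and joining to the Serverinfo game instance.
; BeginPlay caches that instance, then displays WB_MainMenu with cursor and UI-only input.
; A separate event creates the W_Chat widget, which Enter focuses in game-and-UI mode, though nothing here calls that creation.
; The T key only casts the game mode to this controller class, with no follow-up.
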(event `self.ReceiveBeginPlay`
  (bind _returnvalue (`GameplayStatics.GetPlayerController` 0))
  (bind _asserverinfo (cast `/Game/BP/Serverinfo` (`GameplayStatics.GetGameInstance`)))
  (set `self.As Serverinfo` _asserverinfo)
  (`/Engine/EditorBlueprintResources/StandardMacros.IsValid` (stale _returnvalue_2)
    (:`Is Valid`
      _)
    (:`Is Not Valid`
      (bind _returnvalue_2 (`|CreateWidget` "/Game/Widgets/WB_MainMenu.WB_MainMenu_C" (`GameplayStatics.GetPlayerController` 0)))))
  (`UserWidget.AddToViewport` _returnvalue_2 0)
  (set `PlayerController.bShowMouseCursor` true _returnvalue)
  (`WidgetBlueprintLibrary.SetInputMode_UIOnlyEx` _returnvalue _returnvalue_2))

(event `Client Host Session`
  (`/Game/BP/Serverinfo.Host Session` (`self.As Serverinfo`)))

(event `Client Join Session`
  (`/Game/BP/Serverinfo.Join Session` (`self.As Serverinfo`)))

(event `Create ChatWidget`
  ;[1 1 1] Chatting
  (bind _returnvalue (`|CreateWidget` "/Game/Widgets/W_Chat.W_Chat_C"))
  (bind _output_get (set `self.W_chat` _returnvalue))
  (`UserWidget.AddToViewport` _output_get 0))

(event `ShowChat`
  ;[1 1 1] Chatting
  (`WidgetBlueprintLibrary.SetInputMode_GameAndUIEx` self (`self.W_chat`))
  (set `self.bShowMouseCursor` true))

(event `Key|Enter`
  (params (Key :type "Key Structure"))
  ;[1 1 1] Chatting
  (:`Pressed`
    (`self.ShowChat`)))

(event `Key|T`
  (params (Key :type "Key Structure"))
  ;[1 1 1] Chatting
  (:`Pressed`
    (cast `/Game/PlayerControllers/PC_MainMenu` (`GameplayStatics.GetGameMode`))))

(fn `UserConstructionScript`)